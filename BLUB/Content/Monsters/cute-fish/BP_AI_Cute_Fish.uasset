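; BP_AI_Cute_Fish is the AI controller for the cute fish monster, running BT_Cute_Fish on BeginPlay.
; AI perception updates for BP_Player write whether the player is sensed to the CanSeePlayer blackboard key.
; Tick copies IsFedd to the blackboard only while it is true, so this controller never clears that key.
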(event OnTargetPerceptionUpdated(AIPerception)
  (params (Actor :type Actor%20Object%20Reference) (Stimulus :type AI%20Stimulus%20Structure))
  (Utilities|Casting|CastToBP_Player Actor)
  (AI|Components|Blackboard|SetValueasBool (AI|GetBlackboard 0) (Utilities|Name|MakeLiteralName "CanSeePlayer") (.bSuccessfullySensed (Utilities|Struct|BreakAIStimulus Stimulus))))

(event EventBeginPlay
  (AI|RunBehaviorTree "/Game/Monsters/cute-fish/BT_Cute_Fish.BT_Cute_Fish"))

(event EventTick
  (params (DeltaSeconds :type Float%20%28single-precision%29))
  (bind _isfedd (Variables|Default|GetIsFedd))
  (if _isfedd
    (AI|Components|Blackboard|SetValueasBool (AI|GetBlackboard 0) (Utilities|Name|MakeLiteralName "IsFedd") _isfedd)))

(fn ConstructionScript)