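; Flying fish monster that attacks the player on contact and can be fed.
; Box overlap with the player applies damage if CanAttack is set, then halts movement, disables player input and launches them along the fish's forward vector after the animation time.
; Input returns at launch, while flight and attack readiness return after the attack delay.
; Overlapping food instead sets IsFedd on its BP_AI_Cute_Fish controller.
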(event OnComponentBeginOverlap(Box)
  (params (OverlappedComponent :type Primitive%20Component%20Object%20Reference) (OtherActor :type Actor%20Object%20Reference) (OtherComp :type Primitive%20Component%20Object%20Reference) (OtherBodyIndex :type Integer) (bFromSweep :type Boolean) (SweepResult :type Hit%20Result%20Structure%20%28by%20ref%29))
  (bind _asbp_player (Utilities|Casting|CastToBP_Player OtherActor)
    (:then
      (bind _player (CallFunction|TargetPlayer _asbp_player))
      (Pawn|Components|CharacterMovement|DisableMovement (Variables|Character|GetCharacterMovement))
      (Variables|Components|SetcanAttack false)
      (Input|DisableInput _player 0)
      (Utilities|FlowControl|Delay (Variables|Components|GetAnimationTime))
      (Character|LaunchCharacter _player (* (Math|Vector|GetForwardVector (Transformation|GetWorldRotation (Variables|Collision|GetCapsuleComponent self))) 1e+03) false false)
      (Input|EnableInput _player 0)
      (Utilities|FlowControl|Delay (- (Variables|Components|GetAttackDelay) (Variables|Components|GetAnimationTime)))
      (Pawn|Components|CharacterMovement|SetMovementMode (Variables|Character|GetCharacterMovement) "MOVE_Flying" 0)
      (Variables|Components|SetcanAttack true)
      (Development|PrintString "ATTACK READY"))
    (:CastFailed
      (Utilities|Casting|CastToBP_FOOD OtherActor
        (:then
          (Development|PrintString "FOOD")
          (bind _asbp_ai_cute_fish (Utilities|Casting|CastToBP_AI_Cute_Fish (AI|GetAIController self))
            (:then
              (Development|PrintString "Cast AI CUTE" true true "(R=0.289933,G=1.000000,B=0.000000,A=1.000000)" 1e+01)
              (Variables|/Game/Monsters/cute-fish/BP_AI_Cute_Fish.BP_AI_Cute_Fish_C|SetIsFedd _asbp_ai_cute_fish true))
            (:CastFailed
              (Development|PrintString "Cast AI CUTE Failed" true true "(R=1.000000,G=0.028890,B=0.000000,A=1.000000)" 1e+01))))
        (:CastFailed
          (Development|PrintString "NO FOOD"))))))

(event EventBeginPlay
  (Pawn|Components|CharacterMovement|SetMovementMode (Variables|Character|GetCharacterMovement) "MOVE_Flying" 0))

(event Collision|EventActorBeginOverlap
  (params (OtherActor :type Actor%20Object%20Reference)))

(event EventTick
  (params (DeltaSeconds :type Float%20%28single-precision%29)))

(fn ConstructionScript)

(fn TargetPlayer
  (params (Actor :type BP%20Player%20Object%20Reference))
  (bind _self self)
  (Development|PrintString (Utilities|GetDisplayName 0))
  (if (Variables|Components|GetcanAttack)
    (Game|Damage|ApplyDamage Actor 1e+02 (Pawn|GetController _self) _self)
    (Development|PrintString "SHOOT")
    (return Actor)))