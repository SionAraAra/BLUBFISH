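; BP_Ugly_Fish is a flying-mode monster that moves to a StartLocation on BeginPlay and reacts to overlaps on its Box.
; Overlapping a player applies damage if CanAttack is set, freezes fish movement and player input, then launches the player along the fish's forward vector after AnimationTime.
; Movement and attack return after AttackDelay.
; Overlapping BP_FOOD sets IsFedd on its BP_AI_Ugly_Fish controller.
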(event OnComponentBeginOverlap(Box)
  (params (OverlappedComponent :type Primitive%20Component%20Object%20Reference) (OtherActor :type Actor%20Object%20Reference) (OtherComp :type Primitive%20Component%20Object%20Reference) (OtherBodyIndex :type Integer) (bFromSweep :type Boolean) (SweepResult :type Hit%20Result%20Structure%20%28by%20ref%29))
  (bind _asbp_player (Utilities|Casting|CastToBP_Player OtherActor)
    (:then
      (bind _player (CallFunction|TargetPlayer _asbp_player))
      (Pawn|Components|CharacterMovement|DisableMovement (Variables|Character|GetCharacterMovement))
      (Variables|Default|SetcanAttack false)
      (Input|DisableInput _player 0)
      (Utilities|FlowControl|Delay (Variables|Default|GetAnimationTime))
      (Character|LaunchCharacter _player (* (Math|Vector|GetForwardVector (Transformation|GetWorldRotation (Variables|Collision|GetCapsuleComponent self))) 1e+03) false false)
      (Input|EnableInput _player 0)
      (Utilities|FlowControl|Delay (- (Variables|Default|GetAttackDelay) (Variables|Default|GetAnimationTime)))
      (Pawn|Components|CharacterMovement|SetMovementMode (Variables|Character|GetCharacterMovement) "MOVE_Flying" 0)
      (Variables|Default|SetcanAttack true)
      (Development|PrintString "ATTACK READY"))
    (:CastFailed
      (Utilities|Casting|CastToBP_FOOD OtherActor
        (:then
          (Development|PrintString "FOOD")
          (bind _asbp_ai_ugly_fish (Utilities|Casting|CastToBP_AI_Ugly_Fish (AI|GetAIController self))
            (:then
              (Development|PrintString "Cast AI UGLY" true true "(R=0.289933,G=1.000000,B=0.000000,A=1.000000)" 1e+01)
              (Variables|/Game/Monsters/ugly-fish/BP_AI_Ugly_Fish.BP_AI_Ugly_Fish_C|SetIsFedd _asbp_ai_ugly_fish true))
            (:CastFailed
              (Development|PrintString "Cast AI UGLY Failed" true true "(R=1.000000,G=0.028890,B=0.000000,A=1.000000)" 1e+01))))
        (:CastFailed
          (Development|PrintString "NO FOOD"))))))

(event EventBeginPlay
  (Utilities|FlowControl|Sequence
    (:then_0
      (Pawn|Components|CharacterMovement|SetMovementMode (Variables|Character|GetCharacterMovement) "MOVE_Flying" 0))
    (:then_1
      (Transformation|SetActorLocation (Transformation|GetWorldLocation (Variables|/Game/Locations/BP_Monster_Spawn.BP_Monster_Spawn_C|GetDefaultSceneRoot (Variables|Default|GetStartLocation))) false false))))

(event Collision|EventActorBeginOverlap
  (params (OtherActor :type Actor%20Object%20Reference)))

(event EventTick
  (params (DeltaSeconds :type Float%20%28single-precision%29)))

(fn ConstructionScript)

(fn TargetPlayer
  (params (Actor :type BP%20Player%20Object%20Reference))
  (bind _self self)
  (Development|PrintString (Utilities|GetDisplayName 0))
  (if (Variables|Default|GetcanAttack)
    (Game|Damage|ApplyDamage Actor 1e+02 (Pawn|GetController _self) _self)
    (Development|PrintString "SHOOT")
    (return Actor)))